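; BP_SwingBall is a swinging obstacle that knocks the player character into ragdoll.
; From BeginPlay, two timelines drive StaticMesh2's relative pitch, one played forward and the other in reverse.
; Each timeline's Update starts the other through a three-second Delay, so the swing repeats indefinitely.
; A hit on StaticMesh casts the other actor to ThirdPersonCharacter and calls its Ragdoll function.
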(event `self.ReceiveBeginPlay`
  (bind (_direction `_새_트랙_0`) (`Timeline|타임라인_0` :!via `PlayFromStart` :!label _label)
    (:`Update`
      (`SceneComponent.K2_SetRelativeRotation` (`self.StaticMesh2`) (`KismetMathLibrary.MakeRotator` 0.0 `_새_트랙_0`) false false)
      (`KismetSystemLibrary.Delay` 3.0)
      (bind (_direction_2 `_새_트랙_0_2`) (`Timeline|타임라인_1` :!via `ReverseFromEnd`)
        (:`Update`
          (`SceneComponent.K2_SetRelativeRotation` (`self.StaticMesh2`) (`KismetMathLibrary.MakeRotator` 0.0 `_새_트랙_0_2`) false false)
          (`KismetSystemLibrary.Delay` 3.0)
          (goto _label :!via `PlayFromStart`))))))

(event `self.StaticMesh.OnComponentHit`
  (params (HitComponent :type "PrimitiveComponent Object Reference") (OtherActor :type "Actor Object Reference") (OtherComp :type "PrimitiveComponent Object Reference") (NormalImpulse :type "Vector Structure") (Hit :type "HitResult Structure (by ref)"))
  (bind _asthird_person_character (cast `/Game/ThirdPersonBP/Blueprints/ThirdPersonCharacter` OtherActor))
  (`/Game/ThirdPersonBP/Blueprints/ThirdPersonCharacter.Ragdoll` _asthird_person_character))

(fn `UserConstructionScript`)